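; BP_B38 is a player-controllable airplane pawn that flies forward continuously while the player steers its pitch and roll.
; Each Tick spins both propeller components through NewFunction at a NewVar-based rate and applies full forward movement input along the actor's forward vector.
; The pitch and roll input axes add local actor rotation scaled by Speed and delta time.
; An older local-offset movement node remains unconnected and never runs.
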(event `self.ReceiveTick`
  (params (DeltaSeconds :type "Float (single-precision)"))
  (`self.NewFunction` (`self.SM_P38_Propeller`))
  (`self.NewFunction` (`self.SM_P38_Propeller1`))
  (`self.AddMovementInput` (`self.GetActorForwardVector`)))

(event `InputAxis|pitch`
  (params (AxisValue :type "Float (single-precision)"))
  ;[1 0.224 0.224] 피치 회전
  (`self.K2_AddActorLocalRotation` (`KismetMathLibrary.MakeRotator` 0.0 (* AxisValue (`GameplayStatics.GetWorldDeltaSeconds`) (`self.speed`)))))

(event `InputAction|왼쪽 cntl`
  (params (Key :type "Key Structure")))

(event `InputAxis|roll`
  (params (AxisValue :type "Float (single-precision)"))
  ;[1 1 1] 롤회전
  (`self.K2_AddActorLocalRotation` (`KismetMathLibrary.MakeRotator` (* AxisValue (`GameplayStatics.GetWorldDeltaSeconds`) (`self.speed`)))))

(fn `NewFunction`
  (params (self2 :type "SceneComponent Object Reference"))
  (`SceneComponent.K2_AddLocalRotation` self2 (`KismetMathLibrary.MakeRotator` (* (`GameplayStatics.GetWorldDeltaSeconds`) (`self.NewVar`))) false false))

(fn `UserConstructionScript`)